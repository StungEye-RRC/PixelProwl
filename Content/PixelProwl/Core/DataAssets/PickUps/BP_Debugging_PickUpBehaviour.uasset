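; Debug pickup behaviour that reports the details of a pickup and the player character passed with it.
; The Behaviour event stores the player character and data asset, then chains string builders into one on-screen print.
; The message shows the asset, its points, particles and behaviour count, plus the character.
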(event EventBehaviour
  (params (PlayerCharacter :type Player%20Character%20Object%20Reference) (DataAsset :type Pick%20Up%20Data%20Asset%20Object%20Reference))
  (Variables|Default|SetData%20Asset DataAsset)
  (Variables|Default|SetPlayer%20Character PlayerCharacter)
  (Development|PrintString 0 (Utilities|String|BuildString(Object) (Utilities|String|BuildString(Integer) (Utilities|String|BuildString(Object) (Utilities|String|BuildString(Integer) (Utilities|String|BuildString(Object) "" "Pick Up: " (Variables|Default|GetData%20Asset) " ") " Points: " (Variables|/Script/PixelProwl.PickUpDataAsset|GetPoints (Variables|Default|GetData%20Asset)) " ") " Particles: " (Variables|/Script/PixelProwl.PickUpDataAsset|GetParticles (Variables|Default|GetData%20Asset)) " ") " # of Behaviours: " (Utilities|Array|Length (Variables|/Script/PixelProwl.PickUpDataAsset|GetBehaviours (Variables|Default|GetData%20Asset))) " ") " Player Character: " (Variables|Default|GetPlayer%20Character)) true true "(R=0.000000,G=0.660000,B=1.000000,A=1.000000)" 4.0))