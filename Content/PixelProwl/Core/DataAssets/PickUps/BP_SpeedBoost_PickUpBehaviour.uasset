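; Pickup behaviour that gives the player character a temporary speed boost.
; Its Behaviour event saves the character's current max walk speed, doubles it and starts a one-shot timer for the configured duration.
; When the timer fires, UndoSpeedBoost restores the saved speed and prints a debug message.
; The saved speed is overwritten on each activation, with no guard against overlapping boosts.
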(event Custom|Undo%20Speed%20Boost
  (Variables|/Script/Engine.CharacterMovementComponent|SetMaxWalkSpeed (Variables|/Script/Engine.Character|GetCharacterMovement (stale EventBehaviour PlayerCharacter)) (Variables|Default|GetPre%20Boost%20Walk%20Speed))
  (Development|PrintString 0 "Speed Boost Over"))

(event EventBehaviour
  (params (PlayerCharacter :type Player%20Character%20Object%20Reference) (DataAsset :type Pick%20Up%20Data%20Asset%20Object%20Reference))
  (bind _charactermovement (Variables|/Script/Engine.Character|GetCharacterMovement PlayerCharacter))
  (Variables|Default|SetPre%20Boost%20Walk%20Speed (Variables|/Script/Engine.CharacterMovementComponent|GetMaxWalkSpeed _charactermovement))
  (Variables|/Script/Engine.CharacterMovementComponent|SetMaxWalkSpeed _charactermovement (* (Variables|Default|GetPre%20Boost%20Walk%20Speed) 2.0))
  (Utilities|Time|SetTimerbyEvent (delegate Custom|Undo%20Speed%20Boost) (Variables|Default|GetSpeedBoostTimeInSeconds)))